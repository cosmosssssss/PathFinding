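; Grid tile for AI pathfinding toward BP_destination, colored red when blocked or yellow when difficult, though only blocking affects the search.
; The scan box-traces neighboring tiles and records costs in the AI character's arrays: move step, Manhattan grid distance to destination and previous tile's total.
; The path pass picks the cheapest traced neighbor below its remembered cost, colors it green and appends it to the AI's path.
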(event EventBeginPlay
  (bind _outactors (Actor|GetAllActorsOfClass "/Game/BP_destination.BP_destination_C"))
  (Variables|Default|SetRef_Destination (Utilities|Array|Get(acopy) _outactors)))

(event Collision|EventActorBeginOverlap
  (params (OtherActor :type Actor%20Object%20Reference)))

(event EventTick
  (params (DeltaSeconds :type Float%20%28single-precision%29)))

(fn ConstructionScript
  (Utilities|FlowControl|Sequence
    (:then_0
      (if (Variables|Default|GetIsblock)
        (Rendering|Material|SetVectorParameterValueonMaterials (Variables|Default|GetPlane) "Color" "1.000000, 0, 0")))
    (:then_1
      (if (Variables|Default|GetIsDifficultToCorss)
        (Rendering|Material|SetVectorParameterValueonMaterials (Variables|Default|GetPlane) "Color" "1.000000,1.000000, 0")))))

(fn PFUCGetDistanceonBoard
  (params (Target :type Actor%20Object%20Reference))
  (bind _returnvalue (Transformation|GetActorLocation))
  (bind _returnvalue_2 (Transformation|GetActorLocation Target))
  (return (Math|Float|Floor (/ (Math|Float|SnapToGrid(Float) (+ (Math|Float|Absolute(Float) (- (.x _returnvalue) (.x _returnvalue_2))) (Math|Float|Absolute(Float) (- (.y _returnvalue) (.y _returnvalue_2)))) 1e+02) 1e+02))))

(fn PFUCGetBoardTotalMoveCost
  (params (AICharacter :type AI%20Character%20Object%20Reference) (BeforeBoard :type BP%20Board%20Object%20Reference))
  (return (+ (Variables|/Game/TopDownBP/Blueprints/AI_Character.AI_Character_C|GetMoveStep AICharacter) (CallFunction|PFUCGetDistanceonBoard (Variables|Default|GetRef_Destination)) (Utilities|Array|Get(acopy) (Variables|/Game/TopDownBP/Blueprints/AI_Character.AI_Character_C|GetBoardHasScanedTotalMove AICharacter) (Utilities|Array|FindItem (Variables|/Game/TopDownBP/Blueprints/AI_Character.AI_Character_C|GetBoardsScanedResult AICharacter) BeforeBoard)))))

(fn FUCScaneBoardNearby
  (params (AICharacter :type AI%20Character%20Object%20Reference))
  (bind _returnvalue (Transformation|GetActorLocation))
  (LocalVariables|SetRef_AICharacter AICharacter)
  (Components|Activation|SetActive (Variables|Default|GetP_ScanParticle) true true)
  (bind _outhits (Class|KismetSystemLibrary|BoxTraceMultiforObjects (Math|Vector|MakeVector (.x _returnvalue) (.y _returnvalue) 3e+02) (Math|Vector|MakeVector (.x _returnvalue) (.y _returnvalue) 1e+02) "50.000000,50.000000,10.000000" "0,45.000000, 0" (Utilities|Array|MakeArray "ObjectTypeQuery2") false 0 "None" true))
  (for _array_element _outhits
    (bind _asbp_board (Utilities|Casting|CastToBP_board (.HitActor (Collision|BreakHitResult _array_element))))
    (if (not (Variables|BP_board_C|GetIsblock _asbp_board))
      (if (Utilities|Array|ContainsItem (Variables|/Game/TopDownBP/Blueprints/AI_Character.AI_Character_C|GetBoardsScanedResult (LocalVariables|GetRef_AICharacter)) _asbp_board)
        (if (< (CallFunction|PFUCGetBoardTotalMoveCost _asbp_board (LocalVariables|GetRef_AICharacter) self) (Utilities|Array|Get(acopy) (Variables|/Game/TopDownBP/Blueprints/AI_Character.AI_Character_C|GetBoardHasScanedTotalMove (LocalVariables|GetRef_AICharacter)) (Utilities|Array|FindItem (Variables|/Game/TopDownBP/Blueprints/AI_Character.AI_Character_C|GetBoardsScanedResult (LocalVariables|GetRef_AICharacter)) _asbp_board)))
          (Utilities|Array|SetArrayElem (Variables|/Game/TopDownBP/Blueprints/AI_Character.AI_Character_C|GetBoardHasScanedTotalMove (LocalVariables|GetRef_AICharacter)) (Utilities|Array|Get(acopy) (Variables|/Game/TopDownBP/Blueprints/AI_Character.AI_Character_C|GetBoardHasScanedTotalMove (LocalVariables|GetRef_AICharacter)) (Utilities|Array|FindItem (Variables|/Game/TopDownBP/Blueprints/AI_Character.AI_Character_C|GetBoardsScanedResult (LocalVariables|GetRef_AICharacter)) _asbp_board)) (CallFunction|PFUCGetBoardTotalMoveCost _asbp_board (LocalVariables|GetRef_AICharacter) self)))
        (else
          (Utilities|Array|Add (Variables|/Game/TopDownBP/Blueprints/AI_Character.AI_Character_C|GetBoardsScanedRemember (LocalVariables|GetRef_AICharacter)) _asbp_board)
          (Utilities|Array|Add (Variables|/Game/TopDownBP/Blueprints/AI_Character.AI_Character_C|GetBoardsScanedResult (LocalVariables|GetRef_AICharacter)) _asbp_board)
          (Utilities|Array|Add (Variables|/Game/TopDownBP/Blueprints/AI_Character.AI_Character_C|GetBoardHasScanedTotalMove (LocalVariables|GetRef_AICharacter)) (CallFunction|PFUCGetBoardTotalMoveCost _asbp_board (LocalVariables|GetRef_AICharacter) self)))))))

(fn FUCScanPathNearby
  (params (AICharacter :type AI%20Character%20Object%20Reference))
  (bind _returnvalue (Transformation|GetActorLocation))
  (LocalVariables|SetRef_AICharacter AICharacter)
  (bind _outhits (Class|KismetSystemLibrary|BoxTraceMultiforObjects (Math|Vector|MakeVector (.x _returnvalue) (.y _returnvalue) 3e+02) (Math|Vector|MakeVector (.x _returnvalue) (.y _returnvalue) 1e+02) "50.000000,50.000000,10.000000" "0,45.000000, 0" (Utilities|Array|MakeArray "ObjectTypeQuery2") false 0 "None" true))
  (for _array_element _outhits
    (bind _asbp_board (Utilities|Casting|CastToBP_board (.HitActor (Collision|BreakHitResult _array_element))))
    (if (not (Variables|BP_board_C|GetIsblock _asbp_board))
      (if (< (Utilities|Array|Get(acopy) (Variables|/Game/TopDownBP/Blueprints/AI_Character.AI_Character_C|GetBoardHasScanedTotalMove (LocalVariables|GetRef_AICharacter)) (Utilities|Array|FindItem (Variables|/Game/TopDownBP/Blueprints/AI_Character.AI_Character_C|GetBoardsScanedResult (LocalVariables|GetRef_AICharacter)) _asbp_board)) (LocalVariables|GetTotalMoveCostRemember))
        (LocalVariables|SetNextMoveBoardRemember _asbp_board)
        (LocalVariables|SetTotalMoveCostRemember (Utilities|Array|Get(acopy) (Variables|/Game/TopDownBP/Blueprints/AI_Character.AI_Character_C|GetBoardHasScanedTotalMove (LocalVariables|GetRef_AICharacter)) (Utilities|Array|FindItem (Variables|/Game/TopDownBP/Blueprints/AI_Character.AI_Character_C|GetBoardsScanedResult (LocalVariables|GetRef_AICharacter)) _asbp_board))))))
  (Utilities|IsValid (LocalVariables|GetNextMoveBoardRemember)
    (:Is%20Valid
      (Rendering|Material|SetVectorParameterValueonMaterials (Variables|BP_board_C|GetPlane (LocalVariables|GetNextMoveBoardRemember)) "Color" "0,1.000000, 0")
      (Variables|/Game/TopDownBP/Blueprints/AI_Character.AI_Character_C|SetNextMoveBoard (LocalVariables|GetRef_AICharacter) (LocalVariables|GetNextMoveBoardRemember))
      (Utilities|Array|Add (Variables|/Game/TopDownBP/Blueprints/AI_Character.AI_Character_C|GetBoardFindResult (LocalVariables|GetRef_AICharacter)) (LocalVariables|GetNextMoveBoardRemember)))))